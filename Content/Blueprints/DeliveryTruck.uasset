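; Player delivery truck for the Undeliverable game mode, with vehicle driving controls, speed-driven engine sound and an Escape-toggled pause menu.
; Mouse drag and release throws a Tempbox parcel relative to truck yaw, with axis-based velocity and wheel-set pitch.
; Tick aims an arrow at the target building, prompts resets after rollovers, and spills random parcels when a vertical-axis trace misses at speed.
; Messages go to UndeliverableWidget; mouse camera rotation is disconnected.
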(event `self.ReceiveBeginPlay`
  (bind _foundwidgets (`WidgetBlueprintLibrary.GetAllWidgetsOfClass` "/Game/Blueprints/UndeliverableWidget.UndeliverableWidget_C"))
  (set `self.WidgetReference` (`|GetArrayItem` _foundwidgets)))

(event `InputAxisKey|MouseX`
  (params (AxisValue :type "Float (single-precision)"))
  ;[1 1 1] Camera Controll
)

(event `InputAxisKey|MouseY`
  (params (AxisValue :type "Float (single-precision)"))
  ;[1 1 1] Camera Controll
)

(event `Key|LeftMouseButton`
  (params (Key :type "Key Structure"))
  (bind (_locationx _locationy) (`PlayerController.GetMousePosition` (`GameplayStatics.GetPlayerController` 0)))
  (bind (_returnvalue_roll _returnvalue_pitch _returnvalue_yaw) (`KismetMathLibrary.BreakRotator` (`SceneComponent.K2_GetComponentRotation` (`self.Mesh`))))
  (bind (_locationx_2 _locationy_2) (`PlayerController.GetMousePosition` (`GameplayStatics.GetPlayerController` 0)))
  (bind _returnvalue (+ (`self.GetInputAxisKeyValue`) (`self.GetInputAxisKeyValue`)))
  ;[1 1 1] Throw Parcel
  (:`Pressed`
    (set `self.MouseStartPosition` (`KismetMathLibrary.MakeVector` _locationx _locationy)))
  (:`Released`
    (bind _output_get (set `self.MouseEndPosition` (`KismetMathLibrary.MakeVector` _locationx_2 _locationy_2 (`self.AngleThrow`))))
    (bind _returnvalue_2 (`|SpawnActorFromClass` "/Game/Blueprints/Tempbox.Tempbox_C" (`KismetMathLibrary.Conv_VectorToTransform` (`SceneComponent.K2_GetComponentLocation` (`self.Arrow`))) "Undefined" "OverrideRootScale" null null))
    (if (`KismetMathLibrary.InRange_FloatFloat` _returnvalue -6.0 6.0)
      (set `self.ThrowVelocity` _returnvalue)
      (else
        (set `self.ThrowVelocity` 6.0)))
    (bind (_returnvalue_x _returnvalue_y) (`KismetMathLibrary.BreakVector` (`KismetMathLibrary.GreaterGreater_VectorRotator` (`KismetMathLibrary.GetDirectionUnitVector` (`self.MouseStartPosition`) _output_get) (`KismetMathLibrary.MakeRotator` 0.0 0.0 (- _returnvalue_yaw -90.0)))))
    (`/Game/Blueprints/Tempbox.Parcel Throw` _returnvalue_2 (`self.ThrowVelocity`) (`KismetMathLibrary.MakeVector` _returnvalue_x _returnvalue_y (`KismetMathLibrary.DegTan` (`self.AngleThrow`))))))

(event `InputAxis|Throttle`
  (params (AxisValue :type "Float (single-precision)"))
  ;[1 1 1] Vehicle Movement
  (`ChaosVehicleMovementComponent.SetThrottleInput` (`self.VehicleMovementComponent`) AxisValue))

(event `InputAxis|Brake`
  (params (AxisValue :type "Float (single-precision)"))
  ;[1 1 1] Vehicle Movement
  (`ChaosVehicleMovementComponent.SetBrakeInput` (`self.VehicleMovementComponent`) AxisValue))

(event `InputAxisKey|MouseWheelAxis`
  (params (AxisValue :type "Float (single-precision)"))
  ;[1 1 1] Throw Parcel
  ;;[1 1 1] Mouse Scroll set angle of throw
  (if (!= AxisValue 0.0)
    (bind _output_get (set `self.AngleThrow` (+ (`self.AngleThrow`) AxisValue)))
    (if (> _output_get 85.0)
      (set `self.AngleThrow` 85.0)
      (elif (< (`self.AngleThrow`) -10.0)
        (set `self.AngleThrow` -10.0)))))

(event `InputAxis|Steering`
  (params (AxisValue :type "Float (single-precision)"))
  ;[1 1 1] Vehicle Movement
  (`ChaosVehicleMovementComponent.SetSteeringInput` (`self.VehicleMovementComponent`) AxisValue))

(event `InputAction|Handbrake`
  (params (Key :type "Key Structure"))
  (bind _vehiclemovementcomponent (`self.VehicleMovementComponent`))
  ;[1 1 1] Vehicle Movement
  (:`Pressed`
    (`ChaosVehicleMovementComponent.SetHandbrakeInput` _vehiclemovementcomponent true))
  (:`Released`
    (`ChaosVehicleMovementComponent.SetHandbrakeInput` _vehiclemovementcomponent false)))

(event `InputAction|ResetVehicle`
  (params (Key :type "Key Structure"))
  (bind (_returnvalue_roll _returnvalue_pitch _returnvalue_yaw) (`KismetMathLibrary.BreakRotator` (`self.K2_GetActorRotation`)))
  ;[1 1 1] Reset Vehicle
  (:`Pressed`
    (if (not (> (`KismetMathLibrary.VSize` (`self.GetVelocity`)) 50.0))
      (`self.K2_TeleportTo` (+ (`self.K2_GetActorLocation`) (0.0 0.0 300.0)) (`KismetMathLibrary.MakeRotator` 0.0 0.0 _returnvalue_yaw))
      (message `/Game/Blueprints/DriverMessage.ShowMessage` (`self.WidgetReference`) "*&^%!!!! Rolled it again."))))

(event `self.ReceiveTick`
  (params (DeltaSeconds :type "Float (single-precision)"))
  (bind (_returnvalue_x _returnvalue_y) (`KismetMathLibrary.BreakVector` (`self.GetVelocity`)))
  (bind _mesh (`self.Mesh`))
  (bind (_returnvalue_roll _returnvalue_pitch) (`KismetMathLibrary.BreakRotator` (`SceneComponent.K2_GetComponentRotation` (`self.Mesh`))))
  (bind _returnvalue (`SceneComponent.K2_GetComponentLocation` _mesh))
  ;[1 1 1] Event Tick
  (`|ExecutionSequence`
    (:`then_0`
      ;;[1 1 1] SetRPMsOnSoundComponent
      (`AudioComponent.SetFloatParameter` (`self.EngineSound`) "RPM" (`KismetMathLibrary.Abs` (`ChaosVehicleMovementComponent.GetForwardSpeed` (`self.VehicleMovementComponent`))))
      ;;[1 1 1] Displaymessage to reset
      (if (and (< (`KismetMathLibrary.VSize` (`self.GetVelocity`)) 50.0) (or (or (>= _returnvalue_roll 60.0) (<= _returnvalue_roll -60.0)) (or (>= _returnvalue_pitch 60.0) (<= _returnvalue_pitch -60.0))))
        (message `/Game/Blueprints/DriverMessage.ShowMessage` (`self.WidgetReference`) "Press R to reset")))
    (:`then_1`
      (bind _asundeliverable (cast `/Game/Blueprints/Undeliverable` (`GameplayStatics.GetGameMode`)))
      (bind _targetbuilding (`/Game/Blueprints/Undeliverable.TargetBuilding` _asundeliverable)
        (:`then`
          (bind (_returnvalue_roll_2 _returnvalue_pitch_2 _returnvalue_yaw) (`KismetMathLibrary.BreakRotator` (`KismetMathLibrary.FindLookAtRotation` (`SceneComponent.K2_GetComponentLocation` (`self.Mesh`)) (`SceneComponent.K2_GetComponentLocation` (`/Game/Blueprints/Building.Building` _targetbuilding)))))
          (`SceneComponent.K2_SetWorldRotation` (`self.TargetArrowPointer`) (`KismetMathLibrary.MakeRotator` 0.0 0.0 _returnvalue_yaw) false false))
        (:`else`)))
    (:`then_2`
      (bind (_outhit _returnvalue_2) (`KismetSystemLibrary.LineTraceSingle` _returnvalue (+ (* (`KismetMathLibrary.GetUpVector` (`SceneComponent.K2_GetComponentRotation` _mesh)) (`self.maxZ`)) _returnvalue) "TraceTypeQuery1"))
      (if _returnvalue_2
        _
        (elif (or (> (`KismetMathLibrary.Abs` _returnvalue_x) 750.0) (> (`KismetMathLibrary.Abs` _returnvalue_y) 750.0))
          (`self.LooseBoxes`))))))

(event `Key|Escape` :paused true
  (params (Key :type "Key Structure"))
  (bind _returnvalue (`GameplayStatics.GetPlayerController` 0))
  ;[1 1 1] Main Menu
  (:`Pressed`
    (`/Engine/EditorBlueprintResources/StandardMacros.FlipFlop`
      (:`A`
        (bind _returnvalue_2 (`|CreateWidget` "/Game/MainMenu/MainMenuWidget.MainMenuWidget_C"))
        (`UserWidget.AddToViewport` _returnvalue_2 0)
        (`GameplayStatics.SetGamePaused` true)
        (set `PlayerController.bShowMouseCursor` true _returnvalue)
        (`WidgetBlueprintLibrary.SetInputMode_GameAndUIEx` _returnvalue null)
        (`Widget.SetIsEnabled` (`/Game/MainMenu/MainMenuWidget.ResumeButton` _returnvalue_2) true))
      (:`B`
        (`Widget.RemoveFromParent` _returnvalue_2)
        (`GameplayStatics.SetGamePaused` false)
        (set `PlayerController.bShowMouseCursor` false _returnvalue)
        (`WidgetBlueprintLibrary.SetInputMode_GameOnly` _returnvalue)))))

(event `LooseBoxes`
  ;[1 1 1] Drop Parcels
  (`KismetSystemLibrary.RetriggerableDelay` 0.5)
  (set `self.SpawnBoxesNum` (`KismetMathLibrary.RandomInteger` 6))
  (while (>= (`self.SpawnBoxesNum`) 0)
    (bind _returnvalue (`|SpawnActorFromClass` "/Game/Blueprints/Tempbox.Tempbox_C" (`KismetMathLibrary.Conv_VectorToTransform` (`SceneComponent.K2_GetComponentLocation` (`self.RearArrow`))) "Undefined" "OverrideRootScale" null null))
    (bind _result (`/Engine/EditorBlueprintResources/StandardMacros.DecrementInt` (`self.SpawnBoxesNum`))
      (:`  `
        (set `self.SpawnBoxesNum` _result)
        (`/Game/Blueprints/Tempbox.Parcel Throw` _returnvalue 0.5 (0.0 0.0 0.0))
        (`/Game/Blueprints/UndeliverableWidget.ShowMessage` (`self.WidgetReference`) (`KismetArrayLibrary.Array_Random` (`self.StringArryLostItems`)))))))

(fn `UserConstructionScript`)