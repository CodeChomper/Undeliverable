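; Building actor that serves as a scoring target for thrown or dropped Tempbox actors.
; The construction script applies a configurable mesh and positions and sizes a high and a low score trigger box from per-instance variables.
; When a Tempbox overlaps either trigger, the building passes a higher or lower point value to the game mode's score message, but only if flagged as the target building.
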(event `self.HighScoreTrigger.OnComponentBeginOverlap`
  (params (OverlappedComponent :type "PrimitiveComponent Object Reference") (OtherActor :type "Actor Object Reference") (OtherComp :type "PrimitiveComponent Object Reference") (OtherBodyIndex :type Integer) (bFromSweep :type Boolean) (SweepResult :type "HitResult Structure (by ref)"))
  (cast `/Game/Blueprints/Tempbox` OtherActor)
  (`self.BoxHitAScoreZone` 10))

(event `self.LowScoreTrigger.OnComponentBeginOverlap`
  (params (OverlappedComponent :type "PrimitiveComponent Object Reference") (OtherActor :type "Actor Object Reference") (OtherComp :type "PrimitiveComponent Object Reference") (OtherBodyIndex :type Integer) (bFromSweep :type Boolean) (SweepResult :type "HitResult Structure (by ref)"))
  (cast `/Game/Blueprints/Tempbox` OtherActor)
  (`self.BoxHitAScoreZone` 5))

(event `BoxHitAScoreZone`
  (params (AddToScore :type Integer))
  (if (`self.TargetBuilding`)
    (message `/Game/Blueprints/Score.AddScore` (`GameplayStatics.GetGameMode`) AddToScore)))

(fn `UserConstructionScript`
  (bind _highscoretrigger (`self.HighScoreTrigger`))
  (bind _lowscoretrigger (`self.LowScoreTrigger`))
  (`StaticMeshComponent.SetStaticMesh` (`self.Building`) (`self.BuildingMesh`))
  (`SceneComponent.K2_SetRelativeLocation` _highscoretrigger (`self.HSTriggerPosition`) false false)
  (`BoxComponent.SetBoxExtent` _highscoretrigger (`self.HSTriggerExtent`) true)
  (`SceneComponent.K2_SetRelativeLocation` _lowscoretrigger (`self.LSTriggerPosition`) false false)
  (`BoxComponent.SetBoxExtent` _lowscoretrigger (`self.LSTriggerExtent`) true))