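; Player character pawn for on-foot movement, with an E-key interact for getting in and out of the delivery truck.
; The Walk axis moves it along the control yaw and passes its speed to PlayerAnimationClass, while mouse X turns the controller.
; Unpossession hides the capsule and its children and disables collision, and possession restores both.
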(event `InputAxis|Walk`
  (params (AxisValue :type "Float (single-precision)"))
  ;[1 1 1] Move Forward and Back
  (`self.AddMovementInput` (`KismetMathLibrary.GetForwardVector` (`KismetMathLibrary.MakeRotator` 0.0 0.0 (.yaw (`self.GetControlRotation`)))) AxisValue)
  (bind _output_get (set `self.Speed` (`KismetMathLibrary.VSize` (`CharacterMovementComponent.GetLastUpdateVelocity` (`self.CharacterMovement`)))))
  (`/Game/Blueprints/PlayerAnimationClass.UpdateSpeed` (cast `/Game/Blueprints/PlayerAnimationClass` (`SkeletalMeshComponent.GetAnimInstance` (`self.Mesh`)) :!pure true) _output_get))

(event `InputAxis|MouseXAxis`
  (params (AxisValue :type "Float (single-precision)"))
  (`self.AddControllerYawInput` AxisValue))

(event `Key|E`
  (params (Key :type "Key Structure"))
  ;[1 1 1] Get in and out of Delivery Truck
  (:`Pressed`
    (`self.Interact`)))

(event `self.ReceiveUnpossessed`
  (params (OldController :type "Controller Object Reference"))
  (bind _capsulecomponent (`self.CapsuleComponent`))
  ;[1 1 1] Get in and out of Delivery Truck
  (`SceneComponent.SetVisibility` _capsulecomponent false true)
  (`PrimitiveComponent.SetCollisionEnabled` _capsulecomponent "NoCollision"))

(event `self.ReceivePossessed`
  (params (NewController :type "Controller Object Reference"))
  (bind _capsulecomponent (`self.CapsuleComponent`))
  ;[1 1 1] Get in and out of Delivery Truck
  (`SceneComponent.SetVisibility` _capsulecomponent true true)
  (`PrimitiveComponent.SetCollisionEnabled` _capsulecomponent "QueryAndPhysics"))

(fn `UserConstructionScript`)