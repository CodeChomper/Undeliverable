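; Delivery game manager that runs a timed loop of sending the player's DeliveryTruck to randomly chosen Buildings and tracking score.
; Each new target is flagged on the Building, with a time limit scaled from horizontal truck-to-building distance and a buff multiplier.
; Tick counts down that timer and draws a debug arrow from truck to target.
; AddScore rewards on-time deliveries or penalizes late ones with sound feedback, then picks the next target.
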(event `self.ReceiveBeginPlay`
  (bind _returnvalue (`GameplayStatics.GetActorOfClass` "/Game/Blueprints/DeliveryTruck.DeliveryTruck_C"))
  (set `self.PlayerTruck` _returnvalue)
  (`self.FindNewTargetHouse`))

(event `self.ReceiveTick`
  (params (DeltaSeconds :type "Float (single-precision)"))
  (set `self.DeliveryTimeLeft` (- (`self.DeliveryTimeLeft`) DeltaSeconds))
  (`self.DrawDebugLineToHouse`))

(event `FindNewTargetHouse`
  (bind _outactors (`GameplayStatics.GetAllActorsOfClass` "/Game/Blueprints/Building.Building_C"))
  (bind _output_get (set `self.TargetBuilding` (`KismetArrayLibrary.Array_Random` _outactors)))
  (set `/Game/Blueprints/Building.TargetBuilding` true _output_get)
  (set `self.DeliveryTimeLeft` (* (/ (`KismetMathLibrary.VSizeXY` (- (`SceneComponent.K2_GetComponentLocation` (`WheeledVehiclePawn.Mesh` (`self.PlayerTruck`))) (`SceneComponent.K2_GetComponentLocation` (`/Game/Blueprints/Building.Building` (`self.TargetBuilding`))))) 1000.0) (`self.DeliveryBuff`))))

(event `/Game/Blueprints/Score.AddScore`
  (params (AddToScore :type Integer))
  (if (> (`self.DeliveryTimeLeft`) 0.0)
    (set `self.PlayerScore` (+ (`self.PlayerScore`) AddToScore))
    (`GameplayStatics.PlaySound2D` "/Game/Sounds/Coin.Coin" 10.0 1.0 0.0 null null)
    (else
      (set `self.PlayerScore` (- (`self.PlayerScore`) 10))
      (`GameplayStatics.PlaySound2D` "/Game/Sounds/Late.Late" 10.0 1.0 0.0 null null)))
  (set `/Game/Blueprints/Building.TargetBuilding` false (`self.TargetBuilding`))
  (`KismetSystemLibrary.PrintString` "You Scored")
  (`self.FindNewTargetHouse`))

(fn `DrawDebugLineToHouse`
  (`KismetSystemLibrary.DrawDebugArrow` (`SceneComponent.K2_GetComponentLocation` (`WheeledVehiclePawn.Mesh` (`self.PlayerTruck`))) (`SceneComponent.K2_GetComponentLocation` (`/Game/Blueprints/Building.Building` (`self.TargetBuilding`))) 0.0 (struct :`R` 1.0 :`B` 0.064798 :`A` 1.0) 0.0 10.0))

(fn `UserConstructionScript`)